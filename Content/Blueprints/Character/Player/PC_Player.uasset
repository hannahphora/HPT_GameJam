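; Player controller that drives the game's screen flow between main menu, gameplay, pause and victory, and routes player input.
; It opens the main menu paused on BeginPlay; starting the game adds the Enhanced Input mapping, caches the player character and builds the HUD and pause widgets.
; Move, jump and interact inputs are forwarded to the character, while the pause input swaps HUD and pause menu.
; Returning to the menu resets the player through the game mode.
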(event Custom|CE_Unpawed
  ;[1 1 1] Pause
  (Game|SetGamePaused false)
  (Widget|RemovefromParent (Variables|Default|GetPauseMenuWidget))
  (UserInterface|Viewport|AddtoViewport (Variables|Default|GetHUDWidget) 0))

(event Custom|CE_StartGame
  ;[1 1 1] BeginPlay/OnPossess/EventTick
  (Game|SetGamePaused false)
  (Viewport|RemoveAllWidgets)
  (Input|AddMappingContext (PlayerController|LocalPlayerSubsystems|GetEnhancedInputLocalPlayerSubsystem) "/Game/Blueprints/Input/IMC_Player.IMC_Player" 0 "(bIgnoreAllPressedKeysUntilRelease=True,bForceImmediately=False,bNotifyUserSettings=False)")
  (bind _aschar_player (Utilities|Casting|CastToCHAR_Player (Pawn|GetControlledPawn)))
  (Variables|Default|SetPlayerCharacter _aschar_player)
  (bind _returnvalue (UserInterface|CreateWidget "/Game/Blueprints/Widgets/WBP_HUD.WBP_HUD_C" self))
  (bind _output_get (Variables|Default|SetHUDWidget _returnvalue))
  (UserInterface|Viewport|AddtoViewport _output_get 0)
  (bind _returnvalue_2 (UserInterface|CreateWidget "/Game/Blueprints/Widgets/WBP_PauseMenu.WBP_PauseMenu_C" self))
  (Variables|Default|SetPauseMenuWidget _returnvalue_2))

(event Custom|CE_StartMenu
  ;[1 1 1] BeginPlay/OnPossess/EventTick
  (Default|CEResetPlayer (.AsGM%20Main (Utilities|Casting|CastToGM_Main (Game|GetGameMode))))
  (Game|SetGamePaused true)
  (Viewport|RemoveAllWidgets)
  (Variables|Default|SetbShowMouseCursor true)
  (bind _returnvalue (UserInterface|CreateWidget "/Game/Blueprints/Widgets/WBP_MainMenu.WBP_MainMenu_C" self))
  (bind _output_get (Variables|Default|SetMainMenuWidget _returnvalue))
  (Input|SetInputModeGameandUI self _output_get "DoNotLock" false true)
  (UserInterface|Viewport|AddtoViewport (Variables|Default|GetMainMenuWidget) 0))

(event Custom|CE_Victory
  ;[1 1 1] BeginPlay/OnPossess/EventTick
  (Game|SetGamePaused true)
  (Viewport|RemoveAllWidgets)
  (bind _returnvalue (UserInterface|CreateWidget "/Game/Blueprints/Widgets/WBP_Victory.WBP_Victory_C" self))
  (UserInterface|Viewport|AddtoViewport _returnvalue 0))

(event Input|EnhancedActionEvents|EnhancedInputActionIA_Move
  (params (ActionValue :type Float%20%28double-precision%29) (ElapsedSeconds :type Float%20%28double-precision%29) (TriggeredSeconds :type Float%20%28double-precision%29) (InputAction :type Input%20Action%20Object%20Reference :default "/Game/Blueprints/Input/Actions/IA_Move.IA_Move"))
  ;[1 1 1] Move/Jump
  (Default|CEMove (Variables|Default|GetPlayerCharacter) ActionValue))

(event Input|EnhancedActionEvents|EnhancedInputActionIA_Jump
  (params (ActionValue :type Boolean) (ElapsedSeconds :type Float%20%28double-precision%29) (TriggeredSeconds :type Float%20%28double-precision%29) (InputAction :type Input%20Action%20Object%20Reference :default "/Game/Blueprints/Input/Actions/IA_Jump.IA_Jump"))
  (bind _playercharacter (Variables|Default|GetPlayerCharacter))
  ;[1 1 1] Move/Jump
  (:Started
    (Character|Jump _playercharacter))
  (:Canceled
    (Character|StopJumping _playercharacter :!label _label))
  (:Completed
    (goto _label)))

(event Input|EnhancedActionEvents|EnhancedInputActionIA_Pause
  (params (ActionValue :type Boolean) (ElapsedSeconds :type Float%20%28double-precision%29) (TriggeredSeconds :type Float%20%28double-precision%29) (InputAction :type Input%20Action%20Object%20Reference :default "/Game/Blueprints/Input/Actions/IA_Pause.IA_Pause"))
  ;[1 1 1] Pause
  (:Started
    (if (Game|IsGamePaused)
      (Game|SetGamePaused false)
      (Widget|RemovefromParent (Variables|Default|GetPauseMenuWidget))
      (UserInterface|Viewport|AddtoViewport (Variables|Default|GetHUDWidget) 0)
      (else
        (Game|SetGamePaused true)
        (Widget|RemovefromParent (Variables|Default|GetHUDWidget))
        (UserInterface|Viewport|AddtoViewport (Variables|Default|GetPauseMenuWidget) 0)))))

(event Input|EnhancedActionEvents|EnhancedInputActionIA_Interact
  (params (ActionValue :type Boolean) (ElapsedSeconds :type Float%20%28double-precision%29) (TriggeredSeconds :type Float%20%28double-precision%29) (InputAction :type Input%20Action%20Object%20Reference :default "/Game/Blueprints/Input/Actions/IA_Interact.IA_Interact"))
  ;[1 1 1] Move/Jump
  (:Started
    (Default|CEInteract (Variables|Default|GetPlayerCharacter))))

(event EventBeginPlay
  ;[1 1 1] BeginPlay/OnPossess/EventTick
  (Utilities|FlowControl|DelayUntilNextTick)
  (Game|SetGamePaused true)
  (Viewport|RemoveAllWidgets)
  (Variables|Default|SetbShowMouseCursor true)
  (bind _returnvalue (UserInterface|CreateWidget "/Game/Blueprints/Widgets/WBP_MainMenu.WBP_MainMenu_C" self))
  (bind _output_get (Variables|Default|SetMainMenuWidget _returnvalue))
  (Input|SetInputModeGameandUI self _output_get "DoNotLock" false true)
  (UserInterface|Viewport|AddtoViewport (Variables|Default|GetMainMenuWidget) 0))

(fn ConstructionScript)