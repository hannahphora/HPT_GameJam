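; Player controller for gameplay that turns Enhanced Input into player character actions and manages the HUD and pause menu.
; BeginPlay adds the input mapping, caches the character and creates both widgets.
; The pause action toggles a flag that swaps widgets, cursor and input mode and blocks move, jump and crouch, without pausing the world.
; Jump release calls Jump again, as StopJumping is left unconnected.
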(event Input|EnhancedActionEvents|EnhancedInputActionIA_Horizontal
  (params (ActionValue :type Float%20%28double-precision%29) (ElapsedSeconds :type Float%20%28double-precision%29) (TriggeredSeconds :type Float%20%28double-precision%29) (InputAction :type Input%20Action%20Object%20Reference :default "/Game/Blueprints/Input/Actions/IA_Horizontal.IA_Horizontal"))
  ;[1 1 1] Move/Jump/Crouch
  (if (not (Variables|Default|GetbPaused))
    (Default|CEMove (Variables|Default|GetPlayerCharacter) ActionValue)))

(event Input|EnhancedActionEvents|EnhancedInputActionIA_Jump
  (params (ActionValue :type Boolean) (ElapsedSeconds :type Float%20%28double-precision%29) (TriggeredSeconds :type Float%20%28double-precision%29) (InputAction :type Input%20Action%20Object%20Reference :default "/Game/Blueprints/Input/Actions/IA_Jump.IA_Jump"))
  (bind _bpaused (Variables|Default|GetbPaused))
  ;[1 1 1] Move/Jump/Crouch
  (:Started
    (if (not _bpaused)
      (Character|Jump (Variables|Default|GetPlayerCharacter) :!label _label)))
  (:Canceled
    (if (not _bpaused) :!label _label_2
      (goto _label)))
  (:Completed
    (goto _label_2)))

(event Input|EnhancedActionEvents|EnhancedInputActionIA_Pause
  (params (ActionValue :type Boolean) (ElapsedSeconds :type Float%20%28double-precision%29) (TriggeredSeconds :type Float%20%28double-precision%29) (InputAction :type Input%20Action%20Object%20Reference :default "/Game/Blueprints/Input/Actions/IA_Pause.IA_Pause"))
  ;[1 1 1] Pause
  (:Started
    (if (Variables|Default|GetbPaused)
      (Variables|Default|SetbPaused false)
      (Variables|Default|SetbShowMouseCursor false)
      (Input|SetInputModeGameOnly self true)
      (Widget|RemovefromParent (Variables|Default|GetPauseMenuWidget))
      (UserInterface|Viewport|AddtoViewport (Variables|Default|GetHUDWidget) 0)
      (else
        (Variables|Default|SetbPaused true)
        (Variables|Default|SetbShowMouseCursor true)
        (Input|SetInputModeGameandUI self (Variables|Default|GetPauseMenuWidget) "DoNotLock" true true)
        (Widget|RemovefromParent (Variables|Default|GetHUDWidget))
        (UserInterface|Viewport|AddtoViewport (Variables|Default|GetPauseMenuWidget) 0)))))

(event Input|EnhancedActionEvents|EnhancedInputActionIA_Crouch
  (params (ActionValue :type Boolean) (ElapsedSeconds :type Float%20%28double-precision%29) (TriggeredSeconds :type Float%20%28double-precision%29) (InputAction :type Input%20Action%20Object%20Reference :default "/Game/Blueprints/Input/Actions/IA_Crouch.IA_Crouch"))
  (bind _playercharacter (Variables|Default|GetPlayerCharacter))
  (bind _bpaused (Variables|Default|GetbPaused))
  ;[1 1 1] Move/Jump/Crouch
  (:Triggered
    (if (not _bpaused) :!label _label
      (Character|Crouch _playercharacter)))
  (:Started
    (goto _label))
  (:Canceled
    (if (not _bpaused) :!label _label_2
      (Character|UnCrouch _playercharacter)))
  (:Completed
    (goto _label_2)))

(event EventBeginPlay
  ;[1 1 1] BeginPlay/OnPossess/EventTick
  (Variables|Default|SetbShowMouseCursor false)
  (Input|SetInputModeGameOnly self true)
  (Input|AddMappingContext (PlayerController|LocalPlayerSubsystems|GetEnhancedInputLocalPlayerSubsystem) "/Game/Blueprints/Input/IMC_Player.IMC_Player" 0 "(bIgnoreAllPressedKeysUntilRelease=True,bForceImmediately=False,bNotifyUserSettings=False)")
  (bind _asbp_player_character (Utilities|Casting|CastToBP_PlayerCharacter (Pawn|GetControlledPawn)))
  (Variables|Default|SetPlayerCharacter _asbp_player_character)
  (Viewport|RemoveAllWidgets)
  (bind _returnvalue (UserInterface|CreateWidget "/Game/Blueprints/Widgets/HUD/WBP_HUD.WBP_HUD_C" self))
  (bind _output_get (Variables|Default|SetHUDWidget _returnvalue))
  (UserInterface|Viewport|AddtoViewport _output_get 0)
  (bind _returnvalue_2 (UserInterface|CreateWidget "/Game/Blueprints/Widgets/PauseMenu/WBP_PauseMenu.WBP_PauseMenu_C" self))
  (Variables|Default|SetPauseMenuWidget _returnvalue_2))

(fn ConstructionScript)