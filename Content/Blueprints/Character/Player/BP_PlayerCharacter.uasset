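; Player character that moves along the world Y axis and can carry and throw a BP_Lamp.
; CE_Move stores the direction, adds movement input and yaws the mesh to match.
; CE_Interact attaches an overlapping lamp to AttachPoint, or releases the held one with physics, spin and directional velocity, applying opposite recoil to the character.
; On destruction it tells GM_Gameplay to reset the player.
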(event Custom|CE_Move
  (params (Direction :type Float%20%28double-precision%29))
  ;[1 1 1] InputEvents
  (Variables|Default|Setmovement Direction)
  (Pawn|Input|AddMovementInput (Math|Vector|MakeVector 0.0 Direction 0.0) 1.0 false)
  (Transformation|SetRelativeRotation (Variables|Character|GetMesh) (Math|Rotator|MakeRotator 0.0 0.0 (* Direction -9e+01)) false false))

(event Custom|CE_Interact
  (bind _capsulecomponent (Variables|Collision|GetCapsuleComponent))
  (bind _overlappingactors (Collision|GetOverlappingActors _capsulecomponent "/Game/Blueprints/Props/BP_Lamp.BP_Lamp_C" :!class /Script/Engine.PrimitiveComponent))
  (bind _output (Utilities|Array|Get(acopy) _overlappingactors))
  ;[1 1 1] Pickup
  (Utilities|IsValid (Variables|Default|GetLamp)
    (:Is%20Valid
      (Variables|/Game/Blueprints/Props/BP_Lamp.BP_Lamp_C|SetbIsHeld (Variables|Default|GetLamp) false)
      (Transformation|DetachFromActor (Variables|Default|GetLamp) "KeepWorld" "KeepWorld" "KeepWorld")
      (Physics|SetSimulatePhysics (Variables|/Game/Blueprints/Props/BP_Lamp.BP_Lamp_C|GetMesh (Variables|Default|GetLamp)) true)
      (Class|PrimitiveComponent|SetPhysicsAngularVelocityinDegrees (Variables|/Game/Blueprints/Props/BP_Lamp.BP_Lamp_C|GetMesh (Variables|Default|GetLamp)) (Class|KismetMathLibrary|RandomUnitVectorinEllipticalConeinDegrees "0, 0, 0" 3.6e+02 3.6e+02) true "None")
      (Physics|SetPhysicsLinearVelocity (Variables|/Game/Blueprints/Props/BP_Lamp.BP_Lamp_C|GetMesh (Variables|Default|GetLamp)) (Math|Vector|MakeVector 0.0 (* (Variables|Default|Getmovement) 6e+02) (* (.z (Transformation|GetVelocity)) 2.0)) false "None")
      (Variables|Default|SetLamp 0)
      (Variables|/Script/Engine.MovementComponent|SetVelocity (Variables|Character|GetCharacterMovement) (Math|Vector|MakeVector (.x (Variables|/Script/Engine.MovementComponent|GetVelocity (Variables|Character|GetCharacterMovement))) (+ (.y (Variables|/Script/Engine.MovementComponent|GetVelocity (Variables|Character|GetCharacterMovement))) (* (Variables|Default|Getmovement) -8e+02)) (* (.z (Variables|/Script/Engine.MovementComponent|GetVelocity (Variables|Character|GetCharacterMovement))) 1.0))))
    (:Is%20Not%20Valid
      (Utilities|IsValid _output
        (:Is%20Valid
          (bind _asbp_lamp (Utilities|Casting|CastToBP_Lamp _output))
          (Variables|/Game/Blueprints/Props/BP_Lamp.BP_Lamp_C|SetbIsHeld _asbp_lamp true)
          (bind _output_get (Variables|Default|SetLamp _asbp_lamp))
          (Transformation|AttachComponentToComponent _output_get (Variables|Default|GetAttachPoint) "None" "SnapToTarget" "SnapToTarget" "KeepWorld" true))))))

(event EventBeginPlay
  ;[1 1 1] BeginPlay/EventTick
)

(event EventDestroyed
  ;[1 1 1] InputEvents
  (bind _asgm_gameplay (Utilities|Casting|CastToGM_Gameplay (Game|GetGameMode)))
  (Default|ResetPlayer _asgm_gameplay))

(event EventTick
  (params (DeltaSeconds :type Float%20%28single-precision%29))
  ;[1 1 1] BeginPlay/EventTick
)

(fn ConstructionScript)