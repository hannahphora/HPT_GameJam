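; Door prop that sinks downward when it receives a Powered event.
; A DoOnce gates a Timeline that lerps the door's relative Z down by a distance derived from its scale plus a margin.
; CE_Reset stops the Timeline, rewinds it and re-arms the DoOnce; a world-location teleport to the start position is left unwired.
; BeginPlay caches starting locations and applies a per-actor time dilation.
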(event Custom|CE_Reset
  (bind _initlocrel (Variables|Default|GetInitLocRel))
  (Utilities|FlowControl|Sequence
    (:then_0
      (bind _time (Timeline|Timeline Stop)
        (:Update
          (Transformation|SetRelativeLocation (Variables|Default|GetDoor) (Math|Vector|MakeVector (.x _initlocrel) (.y _initlocrel) (Math|Float|Lerp (.z _initlocrel) (- (.z _initlocrel) (+ (* (.z (Variables|/Script/Engine.SceneComponent|GetRelativeScale3D (Variables|Default|GetDoor))) 1e+02) 25.0)) _time)) false false))))
    (:then_1
      (Timeline|Timeline SetNewTime))
    (:then_2
      (Utilities|FlowControl|DoOnce false) ; enters at Reset
    )))

(event EventBeginPlay
  (bind _door (Variables|Default|GetDoor))
  (Variables|Default|SetInitialLocation (Transformation|GetWorldLocation _door))
  (Variables|Default|SetInitLocRel (Variables|/Script/Engine.SceneComponent|GetRelativeLocation _door))
  (Variables|Default|SetCustomTimeDilation (Variables|Default|GettimeDilation)))

(event EventPowered
  (bind _initlocrel (Variables|Default|GetInitLocRel))
  (Utilities|FlowControl|DoOnce false
    (:Completed
      (bind _time (Timeline|Timeline Play)
        (:Update
          (Transformation|SetRelativeLocation (Variables|Default|GetDoor) (Math|Vector|MakeVector (.x _initlocrel) (.y _initlocrel) (Math|Float|Lerp (.z _initlocrel) (- (.z _initlocrel) (+ (* (.z (Variables|/Script/Engine.SceneComponent|GetRelativeScale3D (Variables|Default|GetDoor))) 1e+02) 25.0)) _time)) false false))))))

(fn ConstructionScript)