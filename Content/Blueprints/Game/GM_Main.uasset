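; Main game mode that tracks the player's checkpoint and handles respawning.
; The player's starting location is the initial checkpoint, and checkpoint events overwrite it with the given checkpoint's location.
; On reset, it resets the player character, clears velocity and darkness, triggers interact if a lamp reference is valid, and teleports to the checkpoint at a fixed rotation.
; It then calls reset on every lamp and door in the level.
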(event Custom|CE_ResetPlayer
  (bind _aschar_player (Utilities|Casting|CastToCHAR_Player (Pawn|GetControlledPawn (Game|GetPlayerController 0))))
  (Default|CEReest _aschar_player)
  (Variables|/Script/Engine.MovementComponent|SetVelocity (Pawn|GetMovementComponent _aschar_player) "0, 0, 0")
  (Utilities|IsValid (Variables|/Game/Blueprints/Character/Player/CHAR_Player.CHAR_Player_C|GetLamp _aschar_player)
    (:Is%20Valid
      (Default|CEInteract _aschar_player))
    (:Is%20Not%20Valid
      _))
  (Variables|/Game/Blueprints/Character/Player/CHAR_Player.CHAR_Player_C|SetdarknessPercentage _aschar_player 0.0)
  (Transformation|SetActorTransform _aschar_player (Math|Transform|MakeTransform (Variables|Default|GetCurrentCheckpointPos) "0.000000,90.000000,0.000000" "1.000000,1.000000,1.000000") false true)
  (Utilities|FlowControl|Sequence
    (:then_0
      ;[1 1 1] respawn lamps
      (bind _outactors (Actor|GetAllActorsOfClass "/Game/Blueprints/Props/BP_Lamp.BP_Lamp_C"))
      (for _array_element _outactors
        (Default|CEReset _array_element)))
    (:then_1
      ;[1 1 1] respawn doors
      (bind _outactors_2 (Actor|GetAllActorsOfClass "/Game/Blueprints/Props/BP_Door.BP_Door_C"))
      (for _array_element_2 _outactors_2
        (Default|CEReset _array_element_2)))))

(event Custom|CE_Checkpoint
  (params (checkpoint :type BP%20Checkpoint%20Object%20Reference))
  (Variables|Default|SetCurrentCheckpointPos (Transformation|GetActorLocation checkpoint)))

(event EventBeginPlay
  (bind _output_get (Variables|Default|SetFirstCheckPoint (.location (Transformation|GetActorTransform (Game|GetPlayerCharacter 0)))))
  (Variables|Default|SetCurrentCheckpointPos _output_get))

(event EventTick
  (params (DeltaSeconds :type Float%20%28single-precision%29)))

(fn ConstructionScript)