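; Gameplay game mode that respawns the player at the current checkpoint through its ResetPlayer event.
; When player 0 has a valid pawn, the event destroys it and spawns a new BP_PlayerCharacter at the checkpoint location read from GS_Gameplay.
; PC_Gameplay then possesses the new character and stores it as its PlayerCharacter reference.
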(event Custom|ResetPlayer
  (bind _returnvalue (Game|Player|GetPlayerPawn 0))
  (Utilities|IsValid _returnvalue
    (:Is%20Valid
      (Actor|DestroyActor _returnvalue)
      (bind _aspc_gameplay (Utilities|Casting|CastToPC_Gameplay (Game|GetPlayerController 0)))
      (bind _returnvalue_2 (Game|SpawnActorfromClass "/Game/Blueprints/Character/Player/BP_PlayerCharacter.BP_PlayerCharacter_C" (Math|Transform|MakeTransform (Transformation|GetWorldLocation (Variables|/Game/Blueprints/Props/BP_Checkpoint.BP_Checkpoint_C|GetDefaultSceneRoot (Variables|/Game/Blueprints/Game/Gameplay/GS_Gameplay.GS_Gameplay_C|GetCurrentCheckpoint (.AsGS%20Gameplay (Utilities|Casting|CastToGS_Gameplay (Game|GetGameState)))))) "0, 0, 0" "1.000000,1.000000,1.000000") "Undefined" "MultiplyWithRoot" 0 0))
      (Pawn|Possess _aspc_gameplay _returnvalue_2)
      (Variables|/Game/Blueprints/Character/Player/PC_Gameplay.PC_Gameplay_C|SetPlayerCharacter _aspc_gameplay _returnvalue_2))))

(event EventBeginPlay)

(event EventTick
  (params (DeltaSeconds :type Float%20%28single-precision%29)))

(fn ConstructionScript)